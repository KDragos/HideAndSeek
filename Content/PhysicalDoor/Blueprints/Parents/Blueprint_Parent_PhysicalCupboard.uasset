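; Parent Blueprint for a physics-driven cupboard whose five parts, including three sliding boxes, the player moves with the mouse.
; BeginPlay caches the character and HUD, resets the boxes' positions and enables physics after a short delay.
; A trigger volume gates interaction and the HUD hand icon.
; OpenDoor turns mouse deltas into a character-relative direction via scene and arrow components, then applies that impulse to the named part.
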(event OnComponentBeginOverlap(TriggerOut)
  (params (OverlappedComponent :type Primitive%20Component%20Object%20Reference) (OtherActor :type Actor%20Object%20Reference) (OtherComp :type Primitive%20Component%20Object%20Reference) (OtherBodyIndex :type Integer) (bFromSweep :type Boolean) (SweepResult :type Hit%20Result%20Structure%20%28by%20ref%29))
  (bind _impulsefloatup (Variables|Default|GetImpulseFloatUp))
  (bind _impulsefloatturn (Variables|Default|GetImpulseFloatTurn))
  (bind _returnvalue (Math|Vector|MakeVector _impulsefloatturn _impulsefloatup 0.0))
  (bind _returnvalue_2 (Math|Conversions|RotationFromXVector _returnvalue))
  (bind (_roll _pitch _yaw) (Math|Rotator|BreakRotator _returnvalue_2))
  ;[1 1 1] In this fragment we create a zone of interaction of the Character with a door using a Trigger
  (Variables|Default|SetCollisionTriggerOut true)
  (if (== OtherActor (Variables|Default|GetChar))
    ;[1 1 1] The Gate opens when the Character appears in a zone of interraction with a door
    (Utilities|FlowControl|Gate true) ; enters at Open
  ))

(event OnComponentEndOverlap(TriggerOut)
  (params (OverlappedComponent :type Primitive%20Component%20Object%20Reference) (OtherActor :type Actor%20Object%20Reference) (OtherComp :type Primitive%20Component%20Object%20Reference) (OtherBodyIndex :type Integer))
  (bind _char (Variables|Default|GetChar))
  (bind _impulsefloatup (Variables|Default|GetImpulseFloatUp))
  (bind _impulsefloatturn (Variables|Default|GetImpulseFloatTurn))
  (bind _returnvalue (Math|Vector|MakeVector _impulsefloatturn _impulsefloatup 0.0))
  (bind _returnvalue_2 (Math|Conversions|RotationFromXVector _returnvalue))
  (bind (_roll _pitch _yaw) (Math|Rotator|BreakRotator _returnvalue_2))
  ;[1 1 1] In this fragment we create a zone of interaction of the Character with a door using a Trigger
  (Variables|Default|SetCollisionTriggerOut false)
  (if (== OtherActor _char)
    ;[1 1 1] Here starts the event which disables the rotation lock camera to Character
    (Default|OutCapsule _char)
    ;[1 1 1] The Gate opens when the Character appears in a zone of interraction with a door
    (Utilities|FlowControl|Gate true) ; enters at Close
  ))

(event EventOpenDoor
  (params (MouseValueLookUp :type Float%20%28single-precision%29) (MouseValueTurn :type Float%20%28single-precision%29) (ComponentName :type String))
  ;[1 1 1] This fragment places the values from Character to variables
  (Variables|Default|SetImpulseFloatUp MouseValueLookUp)
  (Variables|Default|SetImpulseFloatTurn MouseValueTurn)
  (Variables|Default|SetComponentName ComponentName)
  ;[1 1 1] The Gate opens when the Character appears in a zone of interraction with a door
  (Utilities|FlowControl|Gate true
    (:Exit
      ;[1 1 1] This fragment is responsible for the hiding "hand" icon, clicking on the door when we are in interaction area.
      (Variables|/Game/PhysicalDoor/Blueprints/PD_FirstPersonHUD.PD_FirstPersonHUD_C|SetVisibleIcon (Variables|Default|GetHUD) false)
      ;[1 1 1] Here the direction of the impulse changes, depending on the Character position and mouse position
      (Transformation|SetWorldRotation (Variables|Default|GetSceneDoor) (Transformation|GetActorRotation (Variables|Default|GetChar)) false false)
      (Transformation|SetRelativeRotation (Variables|Default|GetArrowDoor) (Math|Rotator|MakeRotator (.Roll (Math|Rotator|BreakRotator (Math|Conversions|RotationFromXVector (Math|Vector|MakeVector (Variables|Default|GetImpulseFloatTurn) (Variables|Default|GetImpulseFloatUp) 0.0)))) (.Pitch (Math|Rotator|BreakRotator (Math|Conversions|RotationFromXVector (Math|Vector|MakeVector (Variables|Default|GetImpulseFloatTurn) (Variables|Default|GetImpulseFloatUp) 0.0)))) (+ (.Yaw (Math|Rotator|BreakRotator (Math|Conversions|RotationFromXVector (Math|Vector|MakeVector (Variables|Default|GetImpulseFloatTurn) (Variables|Default|GetImpulseFloatUp) 0.0)))) 9e+01)) false false)
      (Variables|Default|SetDirection (* (Math|Vector|GetForwardVector (Variables|Default|GetArrowDoor)) (Math|Float|Sqrt (+ (Math|Float|Square (Variables|Default|GetImpulseFloatUp)) (Math|Float|Square (Variables|Default|GetImpulseFloatTurn))))))
      ;[1 1 1] Here switching the door with which our Character interacts
      (switch string (Variables|Default|GetComponentName)
        (:Sub1
          ;[1 1 1] Impulse
          (Physics|AddImpulse (Variables|Default|GetSub1) (Variables|Default|GetDirection) "None" false))
        (:Sub2
          (Physics|AddImpulse (Variables|Default|GetSub2) (Variables|Default|GetDirection) "None" false))
        (:Sub3
          (Physics|AddImpulse (Variables|Default|GetSub3) (Variables|Default|GetDirection) "None" false))
        (:Sub4
          (Physics|AddImpulse (Variables|Default|GetSub4) (Variables|Default|GetDirection) "None" false))
        (:Sub5
          (Physics|AddImpulse (Variables|Default|GetSub5) (Variables|Default|GetDirection) "None" false))))))

(event EventBeginPlay
  ;[1 1 1] Here we place the way to our character and HUD in variables for further work with them
  (bind _aspd_first_person_character (Utilities|Casting|CastToPD_FirstPersonCharacter (Game|GetPlayerCharacter 0))
    (:then
      (Variables|Default|SetChar _aspd_first_person_character)
      (bind _aspd_first_person_hud (Utilities|Casting|CastToPD_FirstPersonHUD (HUD|GetHUD (Game|GetPlayerController 0)))
        (:then
          (Variables|Default|SetHUD _aspd_first_person_hud)
          ;[1 1 1] In this fragment the boxes are sent to zero position
          (for _array_element (Utilities|Array|MakeArray (Variables|Default|GetSub3) (Variables|Default|GetSub4) (Variables|Default|GetSub5))
            (CallFunction|StartBoxLocation _array_element))
          ;[1 1 1] This fragment is responsible for enabling collision after the appearance of the Character on stage
          (Collision|SetCollisionEnabled (Variables|Default|GetTriggerOut) "QueryAndPhysics")
          ;[1 1 1] Enable physics
          (Utilities|FlowControl|Delay 0.2)
          (Physics|SetSimulatePhysics (Variables|Default|GetSub1) true))
        (:CastFailed
          (Development|PrintString "FirstPersonHUD in the \"Parent_PhysicalDoor\" Blueprint. Cast Failed" true true "(R=1.000000,G=0.000000,B=0.000000,A=1.000000)" 5.0))))
    (:CastFailed
      (Development|PrintString "FirstPersonCharacter in the \"Parent_PhysicalDoor\" Blueprint. Cast Failed" true true "(R=1.000000,G=0.000000,B=0.000000,A=1.000000)" 5.0))))

(event EventFocus
  ;[1 1 1] This fragment is responsible for showing the "hand" icon at mouse hovering on the door when we are in a interaction area.
  (if (Variables|Default|GetCollisionTriggerOut)
    (Variables|/Game/PhysicalDoor/Blueprints/PD_FirstPersonHUD.PD_FirstPersonHUD_C|SetVisibleIcon (Variables|Default|GetHUD) true)))

(fn ConstructionScript)

(fn StartBoxLocation
  (params (StaticMeshComp :type Static%20Mesh%20Component%20Object%20Reference))
  (bind _relativelocation (Variables|/Script/Engine.SceneComponent|GetRelativeLocation StaticMeshComp))
  (bind (_x _y _z) (Math|Vector|BreakVector _relativelocation))
  ;[1 1 1] This fragment relocates the boxes to the start position
  (Transformation|SetRelativeLocation StaticMeshComp (Math|Vector|MakeVector _x 2e+01 _z) false false))