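; Parent Blueprint for a physics-driven door that the first-person character opens by mouse movement or pushes through hits.
; A trigger gates interaction, and Focus shows the HUD hand icon while it is overlapped.
; Open and Hit inputs unlock the door and apply an impulse directed by character rotation and input values.
; CloseDoor re-arms the lock after a short delay, and Tick constrains the body once the hinge swing reaches a threshold.
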(event OnComponentBeginOverlap(TriggerOut)
  (params (OverlappedComponent :type Primitive%20Component%20Object%20Reference) (OtherActor :type Actor%20Object%20Reference) (OtherComp :type Primitive%20Component%20Object%20Reference) (OtherBodyIndex :type Integer) (bFromSweep :type Boolean) (SweepResult :type Hit%20Result%20Structure%20%28by%20ref%29))
  (bind _impulseup (Variables|Default|GetImpulseUp))
  (bind _impulseturn (Variables|Default|GetImpulseTurn))
  (bind _returnvalue (Math|Vector|MakeVector _impulseturn _impulseup 0.0))
  (bind _returnvalue_2 (Math|Conversions|RotationFromXVector _returnvalue))
  (bind (_roll _pitch _yaw) (Math|Rotator|BreakRotator _returnvalue_2))
  ;[1 1 1] In this fragment we create a zone of interaction of the Character with a door using a Trigger
  (Variables|Default|SetCollisionOutTrigger true)
  (if (== OtherActor (Variables|Default|GetChar))
    ;[1 1 1] The Gate opens when the Character appears in a zone of interraction with a door
    (Utilities|FlowControl|Gate true) ; enters at Open
  ))

(event OnComponentEndOverlap(TriggerOut)
  (params (OverlappedComponent :type Primitive%20Component%20Object%20Reference) (OtherActor :type Actor%20Object%20Reference) (OtherComp :type Primitive%20Component%20Object%20Reference) (OtherBodyIndex :type Integer))
  (bind _impulseup (Variables|Default|GetImpulseUp))
  (bind _impulseturn (Variables|Default|GetImpulseTurn))
  (bind _returnvalue (Math|Vector|MakeVector _impulseturn _impulseup 0.0))
  (bind _returnvalue_2 (Math|Conversions|RotationFromXVector _returnvalue))
  (bind (_roll _pitch _yaw) (Math|Rotator|BreakRotator _returnvalue_2))
  ;[1 1 1] In this fragment we create a zone of interaction of the Character with a door using a Trigger
  (Variables|Default|SetCollisionOutTrigger false)
  (if (== OtherActor (Variables|Default|GetChar))
    (Default|OutCapsule (Variables|Default|GetChar))
    ;[1 1 1] The Gate opens when the Character appears in a zone of interraction with a door
    (Utilities|FlowControl|Gate true) ; enters at Close
  ))

(event EventHit
  (params (ImpulseUp :type Float%20%28single-precision%29) (ImpulseTurn :type Float%20%28single-precision%29) (NameComponent :type String))
  ;[1 1 1] This fragment is responsible for the "push" the door, if we are in front of it
  (Variables|Default|SetImpulseUp ImpulseUp)
  (Variables|Default|SetImpulseTurn ImpulseTurn)
  ;[1 1 1] The Gate opens when the Character appears in a zone of interraction with a door
  (Utilities|FlowControl|Gate true
    (:Exit
      ;[1 1 1] This fragment is responsible for the hiding "hand" icon, clicking on the door when we are in interaction area.
      (Variables|/Game/PhysicalDoor/Blueprints/PD_FirstPersonHUD.PD_FirstPersonHUD_C|SetVisibleIcon (Variables|Default|GetHUD) false)
      ;[1 1 1] Here the physics door turns itself on in case of opening
      (Variables|Default|SetLock false)
      (Class|PrimitiveComponent|SetConstraintMode (Variables|Default|GetSub) "Default")
      ;[1 1 1] Here the direction of the impulse changes, depending on the Character position and mouse position
      (Transformation|SetWorldRotation (Variables|Default|GetSceneArrow) (Transformation|GetActorRotation (Variables|Default|GetChar)) false false)
      (Transformation|SetRelativeRotation (Variables|Default|GetArrowDoor) (Math|Rotator|MakeRotator (.Roll (Math|Rotator|BreakRotator (Math|Conversions|RotationFromXVector (Math|Vector|MakeVector (Variables|Default|GetImpulseTurn) (Variables|Default|GetImpulseUp) 0.0)))) (.Pitch (Math|Rotator|BreakRotator (Math|Conversions|RotationFromXVector (Math|Vector|MakeVector (Variables|Default|GetImpulseTurn) (Variables|Default|GetImpulseUp) 0.0)))) (+ (.Yaw (Math|Rotator|BreakRotator (Math|Conversions|RotationFromXVector (Math|Vector|MakeVector (Variables|Default|GetImpulseTurn) (Variables|Default|GetImpulseUp) 0.0)))) 9e+01)) false false)
      ;[1 1 1] Impulse
      (Physics|AddImpulse (Variables|Default|GetSub) (* (Math|Vector|GetForwardVector (Variables|Default|GetArrowDoor)) (Math|Float|Sqrt (+ (Math|Float|Square (Variables|Default|GetImpulseUp)) (Math|Float|Square (Variables|Default|GetImpulseTurn))))) "None" false))))

(event EventTick
  (params (DeltaSeconds :type Float%20%28single-precision%29))
  ;[1 1 1] Every frame is verified " if the door is locked"
  (if (Variables|Default|GetLock)
    (if (>= (Math|Float|Floor (Class|PhysicsConstraintComponent|GetCurrentSwing1 (Variables|Default|GetPhysicsConstraint))) 48)
      (Class|PrimitiveComponent|SetConstraintMode (Variables|Default|GetSub) "YZPlane"))))

(event EventOpenDoor
  (params (MouseValueLookUp :type Float%20%28single-precision%29) (MouseValueTurn :type Float%20%28single-precision%29) (ComponentName :type String))
  ;[1 1 1] This fragment places the values from Character to variables
  (Variables|Default|SetImpulseUp MouseValueLookUp)
  (Variables|Default|SetImpulseTurn MouseValueTurn)
  ;[1 1 1] The Gate opens when the Character appears in a zone of interraction with a door
  (Utilities|FlowControl|Gate true
    (:Exit
      ;[1 1 1] This fragment is responsible for the hiding "hand" icon, clicking on the door when we are in interaction area.
      (Variables|/Game/PhysicalDoor/Blueprints/PD_FirstPersonHUD.PD_FirstPersonHUD_C|SetVisibleIcon (Variables|Default|GetHUD) false)
      ;[1 1 1] Here the physics door turns itself on in case of opening
      (Variables|Default|SetLock false)
      (Class|PrimitiveComponent|SetConstraintMode (Variables|Default|GetSub) "Default")
      ;[1 1 1] Here the direction of the impulse changes, depending on the Character position and mouse position
      (Transformation|SetWorldRotation (Variables|Default|GetSceneArrow) (Transformation|GetActorRotation (Variables|Default|GetChar)) false false)
      (Transformation|SetRelativeRotation (Variables|Default|GetArrowDoor) (Math|Rotator|MakeRotator (.Roll (Math|Rotator|BreakRotator (Math|Conversions|RotationFromXVector (Math|Vector|MakeVector (Variables|Default|GetImpulseTurn) (Variables|Default|GetImpulseUp) 0.0)))) (.Pitch (Math|Rotator|BreakRotator (Math|Conversions|RotationFromXVector (Math|Vector|MakeVector (Variables|Default|GetImpulseTurn) (Variables|Default|GetImpulseUp) 0.0)))) (+ (.Yaw (Math|Rotator|BreakRotator (Math|Conversions|RotationFromXVector (Math|Vector|MakeVector (Variables|Default|GetImpulseTurn) (Variables|Default|GetImpulseUp) 0.0)))) 9e+01)) false false)
      ;[1 1 1] Impulse
      (Physics|AddImpulse (Variables|Default|GetSub) (* (Math|Vector|GetForwardVector (Variables|Default|GetArrowDoor)) (Math|Float|Sqrt (+ (Math|Float|Square (Variables|Default|GetImpulseUp)) (Math|Float|Square (Variables|Default|GetImpulseTurn))))) "None" false))))

(event EventBeginPlay
  ;[1 1 1] Here we place the way to our character and HUD in variables for further work with them
  (bind _aspd_first_person_character (Utilities|Casting|CastToPD_FirstPersonCharacter (Game|GetPlayerCharacter 0))
    (:then
      (Variables|Default|SetChar _aspd_first_person_character)
      (bind _aspd_first_person_hud (Utilities|Casting|CastToPD_FirstPersonHUD (HUD|GetHUD (Game|GetPlayerController 0)))
        (:then
          (Variables|Default|SetHUD _aspd_first_person_hud)
          ;[1 1 1] This fragment is responsible for enabling collision after the appearance of the Character on stage
          (Collision|SetCollisionEnabled (Variables|Default|GetTriggerOut) "QueryAndPhysics"))
        (:CastFailed
          (Development|PrintString "FirstPersonHUD in the \"Parent_PhysicalDoor\" Blueprint. Cast Failed" true true "(R=1.000000,G=0.000000,B=0.000000,A=1.000000)" 5.0))))
    (:CastFailed
      (Development|PrintString "FirstPersonCharacter in the \"Parent_PhysicalDoor\" Blueprint. Cast Failed" true true "(R=1.000000,G=0.000000,B=0.000000,A=1.000000)" 5.0))))

(event EventFocus
  ;[1 1 1] This fragment is responsible for showing the "hand" icon at mouse hovering on the door when we are in a interaction area.
  (if (Variables|Default|GetCollisionOutTrigger)
    (Variables|/Game/PhysicalDoor/Blueprints/PD_FirstPersonHUD.PD_FirstPersonHUD_C|SetVisibleIcon (Variables|Default|GetHUD) true)))

(event EventCloseDoor
  ;[1 1 1] Door Closed
  (Utilities|FlowControl|Delay 0.01)
  (Variables|Default|SetLock true))

(fn ConstructionScript)