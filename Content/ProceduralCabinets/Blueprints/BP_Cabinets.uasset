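; Base Blueprint for procedural cabinet sets, with child Blueprints supplying per-cabinet configs, shelf lists and door meshes.
; GenerateCabinets chains cabinet meshes through accumulated transforms, adding evenly spaced shelves, an overridable extra-configuration hook and doors.
; Doors follow swing and cabinet type, with configured rotations, hinges, handles and optional glass.
; Dynamic material instances apply wood textures, tint and wear, randomizing texture pan to reduce repetition.
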(event EventBeginPlay)

(event Collision|EventActorBeginOverlap
  (params (OtherActor :type Actor%20Object%20Reference)))

(event EventTick
  (params (DeltaSeconds :type Float%20%28single-precision%29)))

(fn ConstructionScript)

(fn GenerateCabinets
  (params (Number%20of%20Cabinets :type Integer))
  ;[1 1 1] Generate the cabinet set using the configuration in the Cabinets Array
  (for _index (range 0 (- Number%20of%20Cabinets 1))
    (bind _cabinet_base_config (CallFunction|GetCabinetBaseConfig _index))
    ;;[1 1 1] Create Static Mesh Component And Apply Transform
    (bind _returnvalue (AddComponent|AddStaticMeshComponent false))
    (bind _output_get (LocalVariables|SetCurrentMeshComponent _returnvalue))
    (Components|StaticMesh|SetStaticMesh _output_get (.CabinetMesh (Utilities|Struct|BreakSCabinetConfig _cabinet_base_config)))
    (Transformation|AddLocalRotation (LocalVariables|GetCurrentMeshComponent) (LocalVariables|GetCurrentRotation) false false)
    (Transformation|SetRelativeLocation (LocalVariables|GetCurrentMeshComponent) (LocalVariables|GetCurrentLocation) false false)
    ;;[1 1 1] Set Transform For The Next Cabinet
    (LocalVariables|SetCurrentLocation (+ (LocalVariables|GetCurrentLocation) (Math|Vector|RotateVector (.Location (Math|Transform|BreakTransform (.NextCabinetTransform (Utilities|Struct|BreakSCabinetConfig _cabinet_base_config)))) (LocalVariables|GetCurrentRotation))))
    (LocalVariables|SetCurrentRotation (Math|Rotator|CombineRotators (.Rotation (Math|Transform|BreakTransform (.NextCabinetTransform (Utilities|Struct|BreakSCabinetConfig _cabinet_base_config)))) (LocalVariables|GetCurrentRotation)))
    (CallFunction|ConfigureShelves _index _cabinet_base_config (LocalVariables|GetCurrentMeshComponent))
    (CallFunction|ConfigureCabinet _index (LocalVariables|GetCurrentMeshComponent) _cabinet_base_config)
    (CallFunction|ConfigureDoors _index _cabinet_base_config (LocalVariables|GetCurrentMeshComponent))
    (CallFunction|ConfigureMaterial (LocalVariables|GetCurrentMeshComponent) false "NewEnumerator0")))

(fn ConfigureCabinet
  (params (Cabinet%20Index :type Integer) (Staic%20Mesh%20Component :type Static%20Mesh%20Component%20Object%20Reference) (Cabinet%20Config :type S%20Cabinet%20Config%20Structure))
  ;[1 1 1] Extra configuration for the cabinet at the given index. Should be implemented in child blueprints
  (return false))

(fn AttachMeshtoComponent
  (params (Component :type Static%20Mesh%20Component%20Object%20Reference) (Mesh :type Static%20Mesh%20Object%20Reference) (Relative%20Transform :type Transform) (Local%20Transform :type Transform) (Keep%20Relative%20Scale :type Boolean))
  (bind (_location _rotation _scale) (Math|Transform|BreakTransform Local%20Transform))
  (bind _scale_2 (Math|Transform|BreakTransform Relative%20Transform))
  (bind _returnvalue (* _scale _scale_2))
  ;[1 1 1] Helper function for attaching new meshes to existing components
  ;;[1 1 1] Create new static mesh component and attach it to the given one
  (bind _returnvalue_2 (AddComponent|AddStaticMeshComponent false Relative%20Transform))
  (Components|StaticMesh|SetStaticMesh _returnvalue_2 Mesh)
  (Transformation|AttachComponentToComponent _returnvalue_2 Component "None" "KeepRelative" "KeepRelative" "KeepWorld" true)
  ;;[1 1 1] Add Rotation First then the local offset
  (Transformation|AddLocalRotation _returnvalue_2 _rotation false false)
  (Transformation|AddLocalOffset _returnvalue_2 _location false false)
  ;;[1 1 1] Setting the scale
  (if Keep%20Relative%20Scale
    (Transformation|SetRelativeScale3D _returnvalue_2 _returnvalue)
    (else
      (Transformation|SetWorldScale3D _returnvalue_2 _returnvalue)))
  (return _returnvalue_2))

(fn ConfigureShelves
  (params (Cabinet%20Index :type Integer) (Cabinet%20Config :type S%20Cabinet%20Config%20Structure) (Cabinet%20Mesh%20Component :type Static%20Mesh%20Component%20Object%20Reference))
  (bind (_cabinetmesh _shelfmesh _shelfmaxzpos _shelfminzpos) (Utilities|Struct|BreakSCabinetConfig Cabinet%20Config))
  ;[1 1 1] Attaches shelves to the given cabinet with the correct z offsets
  (bind _shelves (CallFunction|GetShelvesforCabinet Cabinet%20Index))
  (for (_array_element _array_index) _shelves
    (bind _new_component (CallFunction|AttachMeshtoComponent :Component Cabinet%20Mesh%20Component :Mesh _shelfmesh :Local%20Transform (Math|Transform|MakeTransform (Math|Vector|MakeVector 0.0 0.0 (+ (Utilities|Struct|BreakSShelfConfig _array_element) (* (+ _array_index 1) (/ (- _shelfmaxzpos _shelfminzpos) (Math|Conversions|ToFloat(Integer) (+ (Utilities|Array|Length _shelves) 1)))) _shelfminzpos)))))
    (CallFunction|ConfigureMaterial _new_component false "NewEnumerator0")))

(fn GetCabinetBaseConfig
  (params (Cabinet%20Index :type Integer))
  ;[1 1 1] Returns the config object for the cabinet at the given index (Must be implemeted in child blueprints)
  (return ""))

(fn GetShelvesforCabinet
  (params (Cabinet%20Index :type Integer))
  ;[1 1 1] Returnes the shelf configuration objects for the cabinet at the given index (must be implemented in child blueprints)
  (return (Utilities|Array|MakeArray "")))

(fn ConfigureDoors
  (params (Cabinet%20Index :type Integer) (Cabinet%20Config :type S%20Cabinet%20Config%20Structure) (Cabinet%20Mesh%20Component :type Static%20Mesh%20Component%20Object%20Reference))
  ;[1 1 1] Add door meshes to the given cabinet with handle and hinges
  (bind _has_doors (CallFunction|HasCabinetDoors Cabinet%20Index))
  (if _has_doors
    (bind _cabinet_instance_config (CallFunction|GetCabinetInstanceConfig Cabinet%20Index))
    (bind (_door_mesh _is_small _is_glass) (CallFunction|GetDoorMeshforCabinet Cabinet%20Index))
    ;;[1 1 1] We add a new door mesh with transform based on its swing direction
    (for (_array_element _array_index) (Utilities|Struct|BreakSCabinetConfig Cabinet%20Config)
      (if (or (== _array_index (Math|Conversions|ToInteger(Byte) (.DoorSwing (Utilities|Struct|BreakSCabinetInstConfig _cabinet_instance_config)))) (Utilities|Enum|Equal(Enum) (.CabinetType (Utilities|Struct|BreakSCabinetInstConfig _cabinet_instance_config)) "NewEnumerator1"))
        (bind _new_component (CallFunction|AttachMeshtoComponent Cabinet%20Mesh%20Component _door_mesh _array_element (Math|Transform|MakeTransform "0, 0, 0" (Math|Rotator|MakeRotator 0.0 0.0 (* (.X (Math|Vector|BreakVector (.Scale (Math|Transform|BreakTransform _array_element)))) (Utilities|Array|Get(acopy) (Utilities|Array|MakeArray (.Door1Rotation (Utilities|Struct|BreakSCabinetInstConfig _cabinet_instance_config)) (.Door2Rotation (Utilities|Struct|BreakSCabinetInstConfig _cabinet_instance_config))) (LocalVariables|GetCurrentDoor))))) false))
        ;;[1 1 1] Adding hinges, handle and set up the door material
        (LocalVariables|SetCurrentDoor (+ (LocalVariables|GetCurrentDoor) 1))
        (CallFunction|AddDoorHinges Cabinet%20Mesh%20Component _new_component (.X (Math|Vector|BreakVector (.Scale (Math|Transform|BreakTransform _array_element)))) _is_small (.CabinetType (Utilities|Struct|BreakSCabinetInstConfig _cabinet_instance_config)))
        (CallFunction|AddDoorHandle _new_component (.DoorHandle (Utilities|Struct|BreakSCabinetInstConfig _cabinet_instance_config)) _is_small)
        (CallFunction|ConfigureMaterial _new_component false "NewEnumerator0")
        ;;[1 1 1] Set up the glass material if the door has glass inset
        (if _is_glass
          (CallFunction|ConfigureGlassforMesh _new_component (.GlassConfig (Utilities|Struct|BreakSCabinetInstConfig _cabinet_instance_config))))))))

(fn GetDoorMeshforCabinet
  (params (Cabinet%20Index :type Integer))
  ;[1 1 1] Returns the door static mesh for the cabinet at the given index (must be implemented in child blueprints)
  (return 0 false false))

(fn GetCabinetInstanceConfig
  (params (Cabinet%20Index :type Integer))
  ;[1 1 1] Returns the config object for the cabinet at the given index (must be implemented in child blueprints)
  (return ""))

(fn HasCabinetDoors
  (params (Cabinet%20Index :type Integer))
  ;[1 1 1] Returns true if the cabinet at the given index has doors (must be implemeted in child blueprints)
  (return false))

(fn GetDoorMeshforCurrentPanelStyle
  (params (Small%20Doors :type Boolean) (Glass%20Doors :type Boolean) (Glass%20Config :type S%20Glass%20Config%20Structure))
  ;[1 1 1] Returns the door static mesh based on the cabinet set door panel style and given parameters
  ;;[1 1 1] Get the door config object for the given door size
  (if Small%20Doors
    (LocalVariables|SetCurrent%20Door%20Configs (Variables|Doors|GetSmall%20Door%20Configs))
    (else
      (LocalVariables|SetCurrent%20Door%20Configs (Variables|Doors|GetDoor%20Configs))))
  ;;[1 1 1] Return the door mesh for the current panel style and glass settings
  (if Glass%20Doors
    (return (.DoorMeshGlass (Utilities|Struct|BreakSCabinetDoorConfig (Utilities|Array|Get(acopy) (LocalVariables|GetCurrent%20Door%20Configs) (Math|Conversions|ToInteger(Byte) (Variables|CabinetSetCommonSettings|GetDoor%20Panel%20Style))))))
    (else
      (return (.DoorMesh (Utilities|Struct|BreakSCabinetDoorConfig (Utilities|Array|Get(acopy) (LocalVariables|GetCurrent%20Door%20Configs) (Math|Conversions|ToInteger(Byte) (Variables|CabinetSetCommonSettings|GetDoor%20Panel%20Style)))))))))

(fn AddDoorHinge
  (params (Cabinet%20Component :type Static%20Mesh%20Component%20Object%20Reference) (Door%20Component :type Static%20Mesh%20Component%20Object%20Reference) (X%20Scale :type Float%20%28single-precision%29) (Relative%20Transform :type Transform) (Cabinet%20Type :type ECabinetType%20Enum))
  ;[1 1 1] Attaches door hinge meshes to cabinet and door components
  ;;[1 1 1] Attach the first hinge to the cabinet component
  (bind _new_component (CallFunction|AttachMeshtoComponent :Component Door%20Component :Mesh "/Game/ProceduralCabinets/Meshes/SM_DoorHingeSmB01.SM_DoorHingeSmB01" :Relative%20Transform Relative%20Transform :Keep%20Relative%20Scale true))
  ;;[1 1 1] Snap the second hinge to the first one
  (bind _returnvalue (AddComponent|AddStaticMeshComponent false))
  (Transformation|SetWorldLocation _returnvalue (Transformation|GetWorldLocation _new_component) false false)
  ;;[1 1 1] Set the scale and rotation for the second hinge and attach it to the door component
  (Transformation|SetRelativeScale3D _returnvalue (Math|Vector|MakeVector X%20Scale 1.0 1.0))
  (if (Utilities|Enum|Equal(Enum) Cabinet%20Type "NewEnumerator2")
    (if (< X%20Scale 0.0)
      (Transformation|AddLocalRotation _returnvalue "0,90.000000, 0" false false)
      (else
        (Transformation|AddLocalRotation _returnvalue "0,0.000000, 0" false false))))
  (Transformation|AttachComponentToComponent _returnvalue Cabinet%20Component "None" "KeepWorld" "KeepRelative" "KeepRelative" true))

(fn AddDoorHinges
  (params (Cabinet%20Component :type Static%20Mesh%20Component%20Object%20Reference) (Door%20Component :type Static%20Mesh%20Component%20Object%20Reference) (X%20Scale :type Float%20%28single-precision%29) (Is%20Small%20Door :type Boolean) (Cabinet%20Type :type ECabinetType%20Enum))
  ;[1 1 1] Attaches 2 door hinges to door and cabinet components with predefined transforms
  ;;[1 1 1] Use different hinge transforms for different door sizes
  (if Is%20Small%20Door
    (LocalVariables|SetHinge%20Transforms (Variables|Doors|GetSmall%20Door%20Hinge%20Transforms))
    (else
      (LocalVariables|SetHinge%20Transforms (Variables|Doors|GetDoor%20Hinge%20Transforms))))
  (for _array_element (LocalVariables|GetHinge%20Transforms)
    (CallFunction|AddDoorHinge Cabinet%20Component Door%20Component X%20Scale _array_element Cabinet%20Type)))

(fn AddDoorHandle
  (params (Door%20Component :type Static%20Mesh%20Component%20Object%20Reference) (Handle%20Type :type EHandleType%20Enum) (Is%20Small%20Door :type Boolean))
  ;[1 1 1] Attaches door handle static mesh belonging to the given handle type to the given door component
  (if (Utilities|Enum|NotEqual(Enum) Handle%20Type "NewEnumerator2")
    (CallFunction|AttachMeshtoComponent :Component Door%20Component :Mesh (Utilities|Array|Get(acopy) (Variables|Handles|GetHandles) (Math|Conversions|ToInteger(Byte) Handle%20Type)) :Relative%20Transform (Utilities|Array|Get(acopy) (Variables|Doors|GetDoor%20Handle%20Transforms) (Math|Conversions|ToInteger(Boolean) Is%20Small%20Door)))))

(fn ConfigureMaterial
  (params (Static%20Mesh%20Component :type Static%20Mesh%20Component%20Object%20Reference) (Override%20Default :type Boolean) (Custom%20Material :type ECabinetMaterial%20Enum) (Custom%20Tint :type Linear%20Color%20Structure) (Material%20index :type Integer))
  ;[1 1 1] Configures the material of the given mesh based on cabinet set settings and given parameters
  ;;[1 1 1] We can use the mesh's default material or a custom one to create the dynamic material instance
  (if Override%20Default
    (LocalVariables|SetCurrent%20Tint Custom%20Tint)
    (LocalVariables|SetCurrent%20Material Custom%20Material)
    (else
      (LocalVariables|SetCurrent%20Tint (Variables|CabinetSetCommonSettings|GetCabinet%20Tint))
      (LocalVariables|SetCurrent%20Material (Variables|CabinetSetCommonSettings|GetCabinet%20Material))))
  (bind _returnvalue (Rendering|Material|CreateDynamicMaterialInstance Static%20Mesh%20Component Material%20index (Utilities|Array|Get(acopy) (Rendering|Material|GetMaterials Static%20Mesh%20Component) Material%20index) :!class /Script/Engine.PrimitiveComponent))
  ;;[1 1 1] Configure texture pan and edge damages
  (Rendering|Material|SetVectorParameterValue _returnvalue "Wood Pan" (Utilities|Struct|MakeLinearColor (Math|Random|RandomFloat) (Math|Random|RandomFloat) 0.0 0.0) :!class /Script/Engine.MaterialInstanceDynamic)
  (Rendering|Material|SetScalarParameterValue _returnvalue "Wear Level" (Math|Conversions|ToFloat(Boolean) (Variables|CabinetSetCommonSettings|GetEdge%20Damages)) :!class /Script/Engine.MaterialInstanceDynamic)
  ;;[1 1 1] Configuring material parameter values using the corresponding material config object and return the dynamic material instance
  (Rendering|Material|SetTextureParameterValue _returnvalue "Wood BaseColor Texture" (.WoodTexture (Utilities|Struct|BreakSCabinetMaterialConfig (Utilities|Array|Get(acopy) (Variables|Default|GetCabinetMaterials) (Math|Conversions|ToInteger(Byte) (LocalVariables|GetCurrent%20Material))))))
  (Rendering|Material|SetTextureParameterValue _returnvalue "Wood Wear Texture" (.WearTexture (Utilities|Struct|BreakSCabinetMaterialConfig (Utilities|Array|Get(acopy) (Variables|Default|GetCabinetMaterials) (Math|Conversions|ToInteger(Byte) (LocalVariables|GetCurrent%20Material))))))
  (Rendering|Material|SetTextureParameterValue _returnvalue "Wood Normal Texture" (.NormalTexture (Utilities|Struct|BreakSCabinetMaterialConfig (Utilities|Array|Get(acopy) (Variables|Default|GetCabinetMaterials) (Math|Conversions|ToInteger(Byte) (LocalVariables|GetCurrent%20Material))))))
  (Rendering|Material|SetTextureParameterValue _returnvalue "Wood Roughenss Texture" (.RoughnessTexture (Utilities|Struct|BreakSCabinetMaterialConfig (Utilities|Array|Get(acopy) (Variables|Default|GetCabinetMaterials) (Math|Conversions|ToInteger(Byte) (LocalVariables|GetCurrent%20Material))))))
  (Rendering|Material|SetScalarParameterValue _returnvalue "Wood Normal Intensity" (.NormalIntensity (Utilities|Struct|BreakSCabinetMaterialConfig (Utilities|Array|Get(acopy) (Variables|Default|GetCabinetMaterials) (Math|Conversions|ToInteger(Byte) (LocalVariables|GetCurrent%20Material))))) :!class /Script/Engine.MaterialInstanceDynamic)
  (Rendering|Material|SetScalarParameterValue _returnvalue "Wood Roughness Min" (.RoughnessMin (Utilities|Struct|BreakSCabinetMaterialConfig (Utilities|Array|Get(acopy) (Variables|Default|GetCabinetMaterials) (Math|Conversions|ToInteger(Byte) (LocalVariables|GetCurrent%20Material))))) :!class /Script/Engine.MaterialInstanceDynamic)
  (Rendering|Material|SetScalarParameterValue _returnvalue "Wood Roughness Max" (.RoughenssMax (Utilities|Struct|BreakSCabinetMaterialConfig (Utilities|Array|Get(acopy) (Variables|Default|GetCabinetMaterials) (Math|Conversions|ToInteger(Byte) (LocalVariables|GetCurrent%20Material))))) :!class /Script/Engine.MaterialInstanceDynamic)
  (Rendering|Material|SetVectorParameterValue _returnvalue "Wood Color" (LocalVariables|GetCurrent%20Tint) :!class /Script/Engine.MaterialInstanceDynamic)
  (return _returnvalue))

(fn ConfigureGlassforMesh
  (params (Mesh :type Static%20Mesh%20Component%20Object%20Reference) (Glass%20Config :type S%20Glass%20Config%20Structure))
  (bind (_frosted _tintglass _glasstint _opacity _ior _roughness) (Utilities|Struct|BreakSGlassConfig Glass%20Config))
  ;[1 1 1] Configures the glass material for the given mesh using the provided glass config
  (bind _returnvalue (Rendering|Material|CreateDynamicMaterialInstance Mesh 1 0 :!class /Script/Engine.PrimitiveComponent))
  ;;[1 1 1] Set each material parameter value using the given glass config object
  (Rendering|Material|SetScalarParameterValue _returnvalue "Opacity" _opacity :!class /Script/Engine.MaterialInstanceDynamic)
  (Rendering|Material|SetScalarParameterValue _returnvalue "IOR" _ior :!class /Script/Engine.MaterialInstanceDynamic)
  (Rendering|Material|SetScalarParameterValue _returnvalue "Roughness" _roughness :!class /Script/Engine.MaterialInstanceDynamic)
  (Rendering|Material|SetVectorParameterValue _returnvalue "Glass Tint" _glasstint :!class /Script/Engine.MaterialInstanceDynamic)
  (Rendering|Material|SetScalarParameterValue _returnvalue "Tint Glass" (Math|Conversions|ToFloat(Boolean) _tintglass) :!class /Script/Engine.MaterialInstanceDynamic)
  (Rendering|Material|SetScalarParameterValue _returnvalue "Frosted" (Math|Conversions|ToFloat(Boolean) _frosted) :!class /Script/Engine.MaterialInstanceDynamic))