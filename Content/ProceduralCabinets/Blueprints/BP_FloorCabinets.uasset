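; Procedural floor cabinet set, a child Blueprint built in the construction script from a per-cabinet config array through GenerateCabinets.
; Getters supply each cabinet's base config, shelves and door mesh, picked by type, model and style.
; ConfigureCabinet attaches drawers with clamped pull-out and handles (doubled on wide cabinets), plus optional countertops.
; Granite countertops get a dynamic M_Granite instance that keeps the mesh's normal texture; wood uses ConfigureMaterial.
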(event EventBeginPlay)

(event Collision|EventActorBeginOverlap
  (params (OtherActor :type Actor%20Object%20Reference)))

(event EventTick
  (params (DeltaSeconds :type Float%20%28single-precision%29)))

(fn ConstructionScript
  ;[1 1 1] Generate the cabinet set using the configuration objects from the Cabinets array
  (|CallParentFunction)
  (CallFunction|GenerateCabinets (Utilities|Array|Length (Variables|Cabinets|GetCabinets))))

(fn ConfigureDrawers
  (params (CabinetIndex :type Integer) (CabinetMeshComponent :type Static%20Mesh%20Component%20Object%20Reference))
  (bind _cabinet_configs (Variables|Config|GetCabinet%20Configs))
  (bind _cabinets (Variables|Cabinets|GetCabinets))
  (bind _door_panel_style (Variables|Default|GetDoor%20Panel%20Style))
  (bind _maxdrawerpull (Variables|Config|GetMaxDrawerPull))
  (bind _item (Utilities|Array|Get(acopy) _cabinets CabinetIndex))
  (bind _returnvalue (Math|Conversions|ToInteger(Byte) _door_panel_style))
  (bind (_baseconfig _cabinetmodel _countertoptype _drawertoppull _drawermiddlepull _drawerbottompull _drawerhandle) (Utilities|Struct|BreakSSCabinetInstConfig_Floor _item))
  (bind _cabinettype (Utilities|Struct|BreakSCabinetInstConfig _baseconfig))
  (bind _returnvalue_2 (Math|Conversions|ToInteger(Byte) _cabinettype))
  (bind _item_2 (Utilities|Array|Get(acopy) _cabinet_configs _returnvalue_2))
  (bind (_baseconfig_2 _drawermeshtop _drawermeshmidbot _drawertoptransform _drawermidtransform _drawerbottransform) (Utilities|Struct|BreakScabinetConfig_Floor _item_2))
  (bind _item_3 (Utilities|Array|Get(acopy) _drawermeshmidbot _returnvalue))
  ;[1 1 1] Adds drawer mesh components with handles and sets the pull out distance for each drawer
  (switch Utilities|FlowControl|Switch|SwitchonECabinetModelFloor _cabinetmodel
    (:NewEnumerator2
      _)
    (:NewEnumerator3
      _))
  ;;[1 1 1] Attach the top drawer to the cabinet component, configure the material and add a handle to it
  (bind _new_component (CallFunction|AttachMeshtoComponent :Component CabinetMeshComponent :Mesh (Utilities|Array|Get(acopy) _drawermeshtop _returnvalue) :Local%20Transform (Math|Transform|ComposeTransforms _drawertoptransform (Math|Transform|MakeTransform (Math|Vector|MakeVector 0.0 (Math|Float|Clamp(Float) _drawertoppull 0.0 _maxdrawerpull) 0.0)))))
  (CallFunction|ConfigureMaterial _new_component false "NewEnumerator0")
  (CallFunction|AddDrawerHandle _new_component _drawerhandle _cabinettype false)
  ;;[1 1 1] If the cabinet type is 'Drawers Only' add the middle and bottom drawers too
  (if (Utilities|Enum|Equal(Enum) _cabinetmodel "NewEnumerator2")
    ;;[1 1 1] Attach the middle drawer to the cabinet component, configure the material and add a handle to it
    (bind _new_component_2 (CallFunction|AttachMeshtoComponent :Component CabinetMeshComponent :Mesh _item_3 :Local%20Transform (Math|Transform|ComposeTransforms _drawermidtransform (Math|Transform|MakeTransform (Math|Vector|MakeVector 0.0 (Math|Float|Clamp(Float) _drawermiddlepull 0.0 _maxdrawerpull) 0.0)))))
    (CallFunction|ConfigureMaterial _new_component_2 false "NewEnumerator0")
    (CallFunction|AddDrawerHandle _new_component_2 _drawerhandle _cabinettype true)
    ;;[1 1 1] Attach the bottom drawer to the cabinet component, configure the material and add a handle to it
    (bind _new_component_3 (CallFunction|AttachMeshtoComponent :Component CabinetMeshComponent :Mesh _item_3 :Local%20Transform (Math|Transform|ComposeTransforms _drawerbottransform (Math|Transform|MakeTransform (Math|Vector|MakeVector 0.0 (Math|Float|Clamp(Float) _drawerbottompull 0.0 _maxdrawerpull) 0.0)))))
    (CallFunction|ConfigureMaterial _new_component_3 false "NewEnumerator0")
    (CallFunction|AddDrawerHandle _new_component_3 _drawerhandle _cabinettype true)))

(fn ConfigureCabinet
  (params (Cabinet%20Index :type Integer) (Staic%20Mesh%20Component :type Static%20Mesh%20Component%20Object%20Reference) (Cabinet%20Config :type S%20Cabinet%20Config%20Structure))
  ;[1 1 1] Configure drawers and the countertop part for the cabinet at the given index
  (CallFunction|ConfigureDrawers Cabinet%20Index Staic%20Mesh%20Component)
  (CallFunction|ConfigureCountertop Staic%20Mesh%20Component Cabinet%20Index)
  (return false))

(fn ConfigureCountertop
  (params (StaticMeshComponent :type Static%20Mesh%20Component%20Object%20Reference) (CabinetIndex :type Integer))
  (bind _cabinet_configs (Variables|Config|GetCabinet%20Configs))
  (bind _cabinets (Variables|Cabinets|GetCabinets))
  (bind _countertop_material (Variables|FloorCabinetSetSettings|GetCountertop%20Material))
  (bind _countertop_tint (Variables|FloorCabinetSetSettings|GetCountertop%20Tint))
  (bind _item (Utilities|Array|Get(acopy) _cabinets CabinetIndex))
  (bind (_baseconfig _cabinetmodel _countertoptype) (Utilities|Struct|BreakSSCabinetInstConfig_Floor _item))
  (bind _cabinettype (Utilities|Struct|BreakSCabinetInstConfig _baseconfig))
  (bind _returnvalue (Math|Conversions|ToInteger(Byte) _countertoptype))
  (bind _returnvalue_2 (Math|Conversions|ToInteger(Byte) _cabinettype))
  (bind _returnvalue_3 (* _returnvalue 3))
  (bind _item_2 (Utilities|Array|Get(acopy) _cabinet_configs _returnvalue_2))
  (bind (_countertopmeshes _countertoptransform) (Utilities|Struct|BreakScabinetConfig_Floor _item_2))
  ;[1 1 1] Configures the countertop section of the cabinet set
  ;;[1 1 1] Do nothing if the cabinet set doesn't have countertop section
  (if (Variables|FloorCabinetSetSettings|GetHas%20Countertop)
    ;;[1 1 1] Get the matching countertop mesh for the cabinet type and attach it to the cabinet component
    (bind _new_component (CallFunction|AttachMeshtoComponent :Component StaticMeshComponent :Mesh (Utilities|Array|Get(acopy) _countertopmeshes _returnvalue) :Local%20Transform _countertoptransform))
    ;;[1 1 1] The countertop material is one of the the 3 wooden material types so we can use the standard 'Configure Material' function
    (if (Utilities|Enum|Equal(Enum) _countertop_material "NewEnumerator3")
      ;;[1 1 1] The countertop material is granite therefore we can't use the standard 'Configure Material' function. We have to set parameter values differently
      (bind _returnvalue_4 (Rendering|Material|CreateDynamicMaterialInstance _new_component _returnvalue_3 0 :!class /Script/Engine.PrimitiveComponent))
      (bind _returnvalue_5 (Rendering|Material|GetTextureParameterValue _returnvalue_4 "Mesh Normal Texture" :!class /Script/Engine.MaterialInstanceDynamic))
      (bind _returnvalue_6 (Rendering|Material|CreateDynamicMaterialInstance _new_component _returnvalue_3 "/Game/ProceduralCabinets/Materials/M_Granite.M_Granite" :!class /Script/Engine.PrimitiveComponent))
      (Rendering|Material|SetVectorParameterValue _returnvalue_6 "Tint Color" _countertop_tint :!class /Script/Engine.MaterialInstanceDynamic)
      (Rendering|Material|SetTextureParameterValue _returnvalue_6 "Mesh Normal Texture" _returnvalue_5)
      (else
        (CallFunction|ConfigureMaterial _new_component true (Utilities|Enum|ByteToEnumECabinetMaterial (Math|Conversions|ToByte(Integer) (Math|Conversions|ToInteger(Byte) _countertop_material))) _countertop_tint _returnvalue_3)))))

(fn GetShelvesforCabinet
  (params (Cabinet%20Index :type Integer))
  ;[1 1 1] Returns the shelf configuration objects for the cabinet at the given index
  (return (.Shelves (Utilities|Struct|BreakSCabinetInstConfig (.BaseConfig (Utilities|Struct|BreakSSCabinetInstConfig_Floor (Utilities|Array|Get(acopy) (Variables|Cabinets|GetCabinets) Cabinet%20Index)))))))

(fn GetCabinetBaseConfig
  (params (Cabinet%20Index :type Integer))
  (bind _cabinets (Variables|Cabinets|GetCabinets))
  (bind _item (Utilities|Array|Get(acopy) _cabinets Cabinet%20Index))
  (bind (_baseconfig _cabinetmodel _countertoptype) (Utilities|Struct|BreakSSCabinetInstConfig_Floor _item))
  ;[1 1 1] Returns the base config object for the cabinet at the given index
  (return (.BaseConfig (Utilities|Struct|BreakScabinetConfig_Floor (Utilities|Array|Get(acopy) (Variables|Config|GetCabinet%20Configs) (+ (Math|Conversions|ToInteger(Byte) (.CabinetType (Utilities|Struct|BreakSCabinetInstConfig _baseconfig))) (* (Math|Conversions|ToInteger(Byte) _countertoptype) 3)))))))

(fn HasCabinetDoors
  (params (Cabinet%20Index :type Integer))
  (bind _cabinets (Variables|Cabinets|GetCabinets))
  (bind _item (Utilities|Array|Get(acopy) _cabinets Cabinet%20Index))
  (bind _cabinetmodel (Utilities|Struct|BreakSSCabinetInstConfig_Floor _item))
  ;[1 1 1] Returns true if the cabinet at the given index has doors
  (return (and (Utilities|Enum|NotEqual(Enum) _cabinetmodel "NewEnumerator0") (Utilities|Enum|NotEqual(Enum) _cabinetmodel "NewEnumerator2"))))

(fn GetCabinetInstanceConfig
  (params (Cabinet%20Index :type Integer))
  ;[1 1 1] Returns the instance config object for the cabinet at the given index
  (return (.BaseConfig (Utilities|Struct|BreakSSCabinetInstConfig_Floor (Utilities|Array|Get(acopy) (Variables|Cabinets|GetCabinets) Cabinet%20Index)))))

(fn GetDoorMeshforCabinet
  (params (Cabinet%20Index :type Integer))
  (bind _cabinet (Utilities|GetCabinetatIndex Cabinet%20Index))
  (bind (_baseconfig _cabinetmodel) (Utilities|Struct|BreakSSCabinetInstConfig_Floor _cabinet))
  (bind (_cabinettype _shelves _doorswing _door1rotation _door2rotation _doorhandle _glassdoors _glassconfig) (Utilities|Struct|BreakSCabinetInstConfig _baseconfig))
  (bind _returnvalue (Utilities|Enum|Equal(Enum) _cabinetmodel "NewEnumerator3"))
  ;[1 1 1] Returns the door mesh for for the cabinet at the given index
  ;;[1 1 1] Get the door mesh for the panel style and return it
  (bind _door_mesh (CallFunction|GetDoorMeshforCurrentPanelStyle _returnvalue _glassdoors _glassconfig))
  (return _door_mesh _returnvalue _glassdoors))

(fn AddDrawerHandle
  (params (Drawer%20Component :type Static%20Mesh%20Component%20Object%20Reference) (Handle%20Type :type EHandleType%20Enum) (Cabinet%20Type :type ECabinetType%20Enum) (Is%20Big%20Drawer :type Boolean))
  (bind _returnvalue (Math|Conversions|ToInteger(Boolean) Is%20Big%20Drawer))
  (bind _returnvalue_2 (Math|Conversions|ToInteger(Byte) Handle%20Type))
  (bind _drawer_handle_transforms (Variables|Drawers|GetDrawer%20Handle%20Transforms))
  (bind _handles (Variables|Default|GetHandles))
  (bind _item (Utilities|Array|Get(acopy) _handles _returnvalue_2))
  (bind _item_2 (Utilities|Array|Get(acopy) _drawer_handle_transforms _returnvalue))
  ;[1 1 1] Sets the handle mesh for the given drawer component
  ;;[1 1 1] Add handle mesh only if the handle type != 'None'
  (if (Utilities|Enum|NotEqual(Enum) Handle%20Type "NewEnumerator2")
    ;;[1 1 1] Attach handle to the drawer component using the correct transform
    (CallFunction|AttachMeshtoComponent :Component Drawer%20Component :Mesh _item :Local%20Transform _item_2)
    ;;[1 1 1] Attach a second handle if the cabinet type is 'Wide'
    (if (Utilities|Enum|Equal(Enum) Cabinet%20Type "NewEnumerator1")
      (CallFunction|AttachMeshtoComponent :Component Drawer%20Component :Mesh _item :Local%20Transform (Math|Transform|ComposeTransforms _item_2 (Math|Transform|MakeTransform (Math|Vector|MakeVector (Variables|Drawers|GetWide%20Drawer%20Handle%202%20Offset) 0.0 0.0)))))))