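; Wall cabinet variant of a procedural cabinet generator, building a configurable set of cabinets in the construction script from its Cabinets array.
; The inherited GenerateCabinets does the work, while this Blueprint supplies per-index shelves, configs, door presence and door meshes.
; Base configs come from CabinetConfigs, indexed by cabinet type with an offset for small cabinets.
; Door meshes follow the panel style, small size and glass options; ConfigureCabinet adds nothing.
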(event EventBeginPlay)

(event Collision|EventActorBeginOverlap
  (params (OtherActor :type Actor%20Object%20Reference)))

(event EventTick
  (params (DeltaSeconds :type Float%20%28single-precision%29)))

(fn ConstructionScript
  ;[1 1 1] Generate the cabinet set using the configuration objects from the Cabinets array
  (|CallParentFunction)
  (CallFunction|GenerateCabinets (Utilities|Array|Length (Variables|Cabinets|GetCabinets))))

(fn ConfigureCabinet
  (params (Cabinet%20Index :type Integer) (Staic%20Mesh%20Component :type Static%20Mesh%20Component%20Object%20Reference) (Cabinet%20Config :type S%20Cabinet%20Config%20Structure))
  ;[1 1 1] For wall cabinets no extra confiuration is needed
  (return false))

(fn GetShelvesforCabinet
  (params (Cabinet%20Index :type Integer))
  ;[1 1 1] Returns the shelf configuration objects for the cabinet at the given index
  (return (.Shelves (Utilities|Struct|BreakSCabinetInstConfig (Utilities|Struct|BreakSSCabinetInstConfig_Wall (Utilities|Array|Get(acopy) (Variables|Cabinets|GetCabinets) Cabinet%20Index))))))

(fn GetCabinetBaseConfig
  (params (Cabinet%20Index :type Integer))
  (bind _cabinets (Variables|Cabinets|GetCabinets))
  (bind _item (Utilities|Array|Get(acopy) _cabinets Cabinet%20Index))
  (bind (_baseconfig _smallcabinet) (Utilities|Struct|BreakSSCabinetInstConfig_Wall _item))
  ;[1 1 1] Returns the base config object for the cabinet at the given index
  (return (Utilities|Struct|BreakScabinetConfig_Wall (Utilities|Array|Get(acopy) (Variables|Config|GetCabinet%20Configs) (+ (Math|Conversions|ToInteger(Byte) (.CabinetType (Utilities|Struct|BreakSCabinetInstConfig _baseconfig))) (* (Math|Conversions|ToInteger(Boolean) _smallcabinet) 3))))))

(fn HasCabinetDoors
  (params (Cabinet%20Index :type Integer))
  ;[1 1 1] Returns true if the cabinet at the given index has doors
  (return (Utilities|Enum|NotEqual(Enum) (.CabinetModel (Utilities|Struct|BreakSSCabinetInstConfig_Wall (Utilities|Array|Get(acopy) (Variables|Cabinets|GetCabinets) Cabinet%20Index))) "NewEnumerator0")))

(fn GetCabinetInstanceConfig
  (params (Cabinet%20Index :type Integer))
  ;[1 1 1] Returns the instance config object for the cabinet at the given index
  (return (.BaseConfig (Utilities|Struct|BreakSSCabinetInstConfig_Wall (Utilities|Array|Get(acopy) (Variables|Cabinets|GetCabinets) Cabinet%20Index)))))

(fn GetDoorMeshforCabinet
  (params (Cabinet%20Index :type Integer))
  (bind _cabinet (Utilities|GetCabinetatIndex Cabinet%20Index))
  (bind (_baseconfig _cabinetmodel _smallcabinet) (Utilities|Struct|BreakSSCabinetInstConfig_Wall _cabinet))
  (bind (_doorswing _door1rotation _door2rotation _doorhandle _glassdoors _glassconfig) (Utilities|Struct|BreakSCabinetInstConfig _baseconfig))
  ;[1 1 1] Returns the door mesh for for the cabinet at the given index
  (bind _door_mesh (CallFunction|GetDoorMeshforCurrentPanelStyle _smallcabinet _glassdoors _glassconfig))
  (return _door_mesh _smallcabinet _glassdoors))