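; A switch actor that starts the VR game when it is opened.
; Open flips the state enum, plays switch and start-looking cues, calls StartGame on MyVRGameMode and plays a timeline that pitches the Switch component.
; Close flips the state back and reverses the timeline; BeginPlay binds it to the game mode's reset-environment event.
; State checks ignore repeated calls, and GetState exposes the current state.
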(event EventOpen
  (if (Utilities|Enum|Equal(Enum) (Variables|Default|GetswitchState) "NewEnumerator1")
    (Variables|Default|SetswitchState "NewEnumerator0")
    (Audio|PlaySoundatLocation "/Game/Audio/siwtchCue.siwtchCue" (Transformation|GetWorldLocation (Variables|Default|GetDefaultSceneRoot)))
    (bind _asmy_vrgame_mode (Utilities|Casting|CastToMyVRGameMode (Game|GetGameMode)))
    (Default|StartGame _asmy_vrgame_mode)
    (Audio|PlaySoundatLocation "/Game/Audio/startLookingCue.startLookingCue" (Transformation|GetWorldLocation (Variables|Default|GetDefaultSceneRoot)))
    (bind _alpha (Timeline|Animation Play)
      (:Update
        (Transformation|SetRelativeRotation (Variables|Default|Getswitch) (Math|Rotator|MakeRotator 0.0 _alpha 0.0) false false)))))

(event EventBeginPlay
  (bind _asmy_vrgame_mode (Utilities|Casting|CastToMyVRGameMode (Game|GetGameMode)))
  (EventDispatchers|BindEventtoResetGameEnvironment _asmy_vrgame_mode (delegate EventClose)))

(event EventClose
  (if (Utilities|Enum|Equal(Enum) (Variables|Default|GetswitchState) "NewEnumerator0")
    (Variables|Default|SetswitchState "NewEnumerator1")
    (Audio|PlaySoundatLocation "/Game/Audio/siwtchCue.siwtchCue" (Transformation|GetWorldLocation (Variables|Default|GetDefaultSceneRoot)))
    (bind _alpha (Timeline|Animation Reverse)
      (:Update
        (Transformation|SetRelativeRotation (Variables|Default|Getswitch) (Math|Rotator|MakeRotator 0.0 _alpha 0.0) false false)))))

(fn ConstructionScript)

(fn GetState
  (return (Variables|Default|GetswitchState)))