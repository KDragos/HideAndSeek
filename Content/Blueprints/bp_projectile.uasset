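; Teleport projectile that moves player pawn 0 to the spot where it lands, apparently for VR locomotion.
; On mesh hit, it accepts only components tagged Floor whose impact point projects to a valid navmesh location.
; A valid hit sets the pawn to the projected point without sweeping and sets the tracking origin to floor level.
; The projectile destroys itself on any hit, valid or not.
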(event OnComponentHit(StaticMeshComponent)
  (params (HitComponent :type Primitive%20Component%20Object%20Reference) (OtherActor :type Actor%20Object%20Reference) (OtherComp :type Primitive%20Component%20Object%20Reference) (NormalImpulse :type Vector) (Hit :type Hit%20Result%20Structure%20%28by%20ref%29))
  (bind _impactpoint (Collision|BreakHitResult Hit))
  (bind _returnvalue (AI|Navigation|ProjectPointtoNavigation _impactpoint 0 0 "0, 0, 0"))
  ;[1 1 1] Destroys the projectile if it hits something that's not the floor or if it's not a valid point of the navmesh
  (if (Components|ComponentHasTag OtherComp "Floor")
    (if (AI|IsValidAILocation _returnvalue)
      (Transformation|SetActorLocation (Game|Player|GetPlayerPawn 0) _returnvalue false false)
      (Class|HeadMountedDisplayFunctionLibrary|SetTrackingOrigin "Floor")
      (Actor|DestroyActor)
      (else
        (Actor|DestroyActor :!label _label)))
    (else
      (goto _label))))

(fn ConstructionScript)