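; Door actor that swings open and closed through its Open and Close events, with a GetState function exposing its current state.
; A two-value state enum guards both events, and one timeline drives the door component's relative yaw, playing forward to open and reversing to close.
; The open sound plays as opening starts, while the close sound waits until the timeline finishes in the closed state.
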(event EventOpen
  (if (Utilities|Enum|Equal(Enum) (Variables|Default|GetdoorState) "NewEnumerator1")
    (Variables|Default|SetdoorState "NewEnumerator0")
    (Audio|PlaySoundatLocation "/Game/Audio/doorOpenCue.doorOpenCue" (Transformation|GetWorldLocation (Variables|Default|GetDoor)))
    (bind _doorrotation (Timeline|doorRotationAnim Play)
      (:Update
        (Transformation|SetRelativeRotation (Variables|Default|GetDoor) (Math|Rotator|MakeRotator 0.0 0.0 _doorrotation) false false))
      (:Finished
        (if (Utilities|Enum|Equal(Enum) (Variables|Default|GetdoorState) "NewEnumerator1")
          (Audio|PlaySoundatLocation "/Game/Audio/doorCloseCue.doorCloseCue" (Transformation|GetWorldLocation (Variables|Default|GetDoor))))))))

(event EventClose
  (if (Utilities|Enum|Equal(Enum) (Variables|Default|GetdoorState) "NewEnumerator0")
    (Variables|Default|SetdoorState "NewEnumerator1")
    (bind _doorrotation (Timeline|doorRotationAnim Reverse)
      (:Update
        (Transformation|SetRelativeRotation (Variables|Default|GetDoor) (Math|Rotator|MakeRotator 0.0 0.0 _doorrotation) false false))
      (:Finished
        (if (Utilities|Enum|Equal(Enum) (Variables|Default|GetdoorState) "NewEnumerator1")
          (Audio|PlaySoundatLocation "/Game/Audio/doorCloseCue.doorCloseCue" (Transformation|GetWorldLocation (Variables|Default|GetDoor))))))))

(fn ConstructionScript)

(fn GetState
  (return (Variables|Default|GetdoorState)))