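; VR game mode that runs a collectible game by managing the active collectible and the score.
; BeginPlay caches every Bp_spawnSpot in the level, and StartGame spawns a Bp_collectible at a random one, keeping a reference to it.
; EndGame destroys that collectible and clears the reference.
; IncreaseScore and GetGameScore expose the score for other Blueprints to increment and read.
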(event Custom|IncreaseScore
  ;[1 1 1] Increase our game score.
  (Math|Float|IncrementFloat (Variables|Default|GetScore)))

(event Custom|EndGame
  ;[1 1 1] If we end the game, the collectible is destroyed and the variable cleared.
  (Utilities|IsValid (Variables|Default|GetactiveCollectible)
    (:Is%20Valid
      (Actor|DestroyActor (Variables|Default|GetactiveCollectible))
      (Variables|Default|SetactiveCollectible 0))))

(event Custom|StartGame
  (bind _possiblespawnlocations (Variables|Default|GetpossibleSpawnLocations))
  ;[1 1 1] When the game is started, a spot is chosen at random for the collectible to spawn. We save the collectible in case we decide to end early.
  (bind _returnvalue (Game|SpawnActorfromClass "/Game/Blueprints/bp_collectible.bp_collectible_C" (Transformation|GetActorTransform (Utilities|Array|Get(acopy) _possiblespawnlocations (Math|Random|RandomInteger (Utilities|Array|Length _possiblespawnlocations)))) "Undefined" 0 0))
  (Variables|Default|SetactiveCollectible _returnvalue))

(event EventBeginPlay
  ;[1 1 1] At the start of the game, we get all our possible spawn spots and save them to a variable
  (bind _outactors (Actor|GetAllActorsOfClass "/Game/Blueprints/bp_spawnSpot.bp_spawnSpot_C"))
  (Variables|Default|SetpossibleSpawnLocations _outactors))

(fn ConstructionScript)

(fn GetGameScore
  (return (Variables|Default|GetScore)))