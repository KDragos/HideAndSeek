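; Goal point actor with an animated flag, where delivered collectibles are consumed and replaced.
; On BeginPlay it spawns a collectible at a random spawn spot actor's transform and starts a timeline that drives the skeletal mesh's relative scale and rotation.
; When a collectible overlaps the box trigger, it is destroyed and a new one is hidden at another randomly picked spot.
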(event OnComponentBeginOverlap(BoxTrigger)
  (params (OverlappedComponent :type Primitive%20Component%20Object%20Reference) (OtherActor :type Actor%20Object%20Reference) (OtherComp :type Primitive%20Component%20Object%20Reference) (OtherBodyIndex :type Integer) (bFromSweep :type Boolean) (SweepResult :type Hit%20Result%20Structure%20%28by%20ref%29))
  (bind _asbp_collectible (Utilities|Casting|CastTobp_collectible OtherActor))
  (Actor|DestroyActor _asbp_collectible)
  (CallFunction|HideCollectible))

(event Custom|HideCollectible
  (bind _outactors (Actor|GetAllActorsOfClass "/Game/bp_spawnSpot.bp_spawnSpot_C"))
  (Game|SpawnActorfromClass "/Game/Blueprints/bp_collectible.bp_collectible_C" (Transformation|GetActorTransform (Utilities|Array|Get(acopy) _outactors (Math|Random|RandomInteger (Utilities|Array|Length _outactors)))) "Undefined" 0 0))

(event EventBeginPlay
  (CallFunction|HideCollectible)
  ;[1 1 1] Animation loop for flag.
  (bind (_direction _alpha _rotation) (Timeline|animation Play)
    (:Update
      (Transformation|SetRelativeScale3D (Variables|SkeletalMeshActor|GetSkeletalMeshComponent) (Math|Vector|Lerp(Vector) (Variables|Default|GetstartingScale) (Variables|Default|GetendingScale) _alpha))
      (Transformation|SetRelativeRotation (Variables|SkeletalMeshActor|GetSkeletalMeshComponent) (Math|Rotator|Lerp(Rotator) (Variables|Default|GetstartingRotation) (Variables|Default|GetendingRotation) _rotation) false false))))

(fn ConstructionScript)