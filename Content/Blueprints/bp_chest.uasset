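; Chest actor for a VR game with a lid that opens and closes, with sound cues.
; Open and Close flip an open/closed state enum, exposed through GetState, and play or reverse the Move timeline that drives the lid's roll.
; The open sound plays as motion starts, while the close sound waits until the reversed timeline finishes.
; On BeginPlay, Close binds to the VR game mode's environment reset.
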(event EventOpen
  ;[1 1 1] Opens and closes the chest. (Plays the animation.)
  (if (Utilities|Enum|Equal(Enum) (Variables|Default|GetopenAbleState) "NewEnumerator1")
    (Variables|Default|SetopenAbleState "NewEnumerator0")
    (Audio|PlaySoundatLocation "/Game/Audio/chestOpenCue.chestOpenCue" (Transformation|GetWorldLocation (Variables|Default|GetboxTop)))
    (bind _alpha (Timeline|Move Play)
      (:Update
        (Transformation|SetRelativeRotation (Variables|Default|GetboxTop) (Math|Rotator|MakeRotator _alpha 0.0 0.0) false false))
      (:Finished
        (if (Utilities|Enum|Equal(Enum) (Variables|Default|GetopenAbleState) "NewEnumerator1")
          (Audio|PlaySoundatLocation "/Game/Audio/chestCloseCue.chestCloseCue" (Transformation|GetWorldLocation (Variables|Default|GetboxTop))))))))

(event EventBeginPlay
  ;[1 1 1] Opens and closes the chest. (Plays the animation.)
  (bind _asmy_vrgame_mode (Utilities|Casting|CastToMyVRGameMode (Game|GetGameMode)))
  (EventDispatchers|BindEventtoResetGameEnvironment _asmy_vrgame_mode (delegate EventClose)))

(event EventClose
  ;[1 1 1] Opens and closes the chest. (Plays the animation.)
  (if (Utilities|Enum|Equal(Enum) (Variables|Default|GetopenAbleState) "NewEnumerator0")
    (Variables|Default|SetopenAbleState "NewEnumerator1")
    (bind _alpha (Timeline|Move Reverse)
      (:Update
        (Transformation|SetRelativeRotation (Variables|Default|GetboxTop) (Math|Rotator|MakeRotator _alpha 0.0 0.0) false false))
      (:Finished
        (if (Utilities|Enum|Equal(Enum) (Variables|Default|GetopenAbleState) "NewEnumerator1")
          (Audio|PlaySoundatLocation "/Game/Audio/chestCloseCue.chestCloseCue" (Transformation|GetWorldLocation (Variables|Default|GetboxTop))))))))

(fn ConstructionScript)

(fn GetState
  (return (Variables|Default|GetopenAbleState)))