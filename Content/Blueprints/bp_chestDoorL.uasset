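; Left chest door Blueprint that swings its ChestDoor component open and closed and tracks an open/closed state, exposed through GetState.
; Open and Close flip that state and play or reverse one Timeline, whose Alpha output sets the door's relative yaw directly.
; The open sound plays as the swing starts, while the close sound plays when the reversed Timeline finishes.
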(event EventOpen
  (if (Utilities|Enum|Equal(Enum) (Variables|Default|GetopenAbleState) "NewEnumerator1")
    (Variables|Default|SetopenAbleState "NewEnumerator0")
    (Audio|PlaySoundatLocation "/Game/Audio/doorOpenCue.doorOpenCue" (Transformation|GetWorldLocation (Variables|Default|GetchestDoor)))
    (bind _alpha (Timeline|Timeline_0 Play)
      (:Update
        (Transformation|SetRelativeRotation (Variables|Default|GetchestDoor) (Math|Rotator|MakeRotator 0.0 0.0 _alpha) false false))
      (:Finished
        (if (Utilities|Enum|Equal(Enum) (Variables|Default|GetopenAbleState) "NewEnumerator1")
          (Audio|PlaySoundatLocation "/Game/Audio/doorCloseCue.doorCloseCue" (Transformation|GetWorldLocation (Variables|Default|GetchestDoor))))))))

(event EventClose
  (if (Utilities|Enum|Equal(Enum) (Variables|Default|GetopenAbleState) "NewEnumerator0")
    (Variables|Default|SetopenAbleState "NewEnumerator1")
    (bind _alpha (Timeline|Timeline_0 Reverse)
      (:Update
        (Transformation|SetRelativeRotation (Variables|Default|GetchestDoor) (Math|Rotator|MakeRotator 0.0 0.0 _alpha) false false))
      (:Finished
        (if (Utilities|Enum|Equal(Enum) (Variables|Default|GetopenAbleState) "NewEnumerator1")
          (Audio|PlaySoundatLocation "/Game/Audio/doorCloseCue.doorCloseCue" (Transformation|GetWorldLocation (Variables|Default|GetchestDoor))))))))

(fn ConstructionScript)

(fn GetState
  (return (Variables|Default|GetopenAbleState)))