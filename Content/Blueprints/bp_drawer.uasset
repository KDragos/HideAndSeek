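; Drawer Blueprint that slides its ChestDoor component open and closed with sound.
; BeginPlay caches the component's relative start position and an end position offset along local Y.
; Open and Close check and flip an enum state, play a cue at the door, and run one timeline forward or in reverse to lerp between those positions.
; GetState exposes the current state.
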(event EventOpen
  (if (Utilities|Enum|Equal(Enum) (Variables|Default|GetopenAbleState) "NewEnumerator1")
    (Variables|Default|SetopenAbleState "NewEnumerator0")
    (Audio|PlaySoundatLocation "/Game/Audio/drawerOpenCue.drawerOpenCue" (Transformation|GetWorldLocation (Variables|Default|GetchestDoor)))
    (bind _alpha (Timeline|Timeline_0 Play)
      (:Update
        (Transformation|SetRelativeLocation (Variables|Default|GetchestDoor) (Math|Vector|Lerp(Vector) (Variables|Default|GetstartPoint) (Variables|Default|GetendPoint) _alpha) false false)))))

(event EventBeginPlay
  (bind _chestdoor (Variables|Default|GetchestDoor))
  (bind _relativelocation (Variables|/Script/Engine.SceneComponent|GetRelativeLocation _chestdoor))
  (Variables|Default|SetstartPoint _relativelocation)
  (Variables|Default|SetendPoint (+ _relativelocation "0.000000,2.500000, 0")))

(event EventClose
  (if (Utilities|Enum|Equal(Enum) (Variables|Default|GetopenAbleState) "NewEnumerator0")
    (Variables|Default|SetopenAbleState "NewEnumerator1")
    (Audio|PlaySoundatLocation "/Game/Audio/drawerCloseCue.drawerCloseCue" (Transformation|GetWorldLocation (Variables|Default|GetchestDoor)))
    (bind _alpha (Timeline|Timeline_0 Reverse)
      (:Update
        (Transformation|SetRelativeLocation (Variables|Default|GetchestDoor) (Math|Vector|Lerp(Vector) (Variables|Default|GetstartPoint) (Variables|Default|GetendPoint) _alpha) false false)))))

(fn ConstructionScript)

(fn GetState
  (return (Variables|Default|GetopenAbleState)))